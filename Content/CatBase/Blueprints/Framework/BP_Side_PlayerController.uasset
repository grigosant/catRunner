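; Side-view player controller that handles the pause menu.
; On BeginPlay it adds the menu Enhanced Input mapping context and focuses the game viewport.
; The menu input toggles pause by creating or removing the pause widget and switching cursor and input mode between UI and game.
; The widget's Continue and Restart are bound to controller events, with restart forwarded to the game mode as a message.
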(event `self.ReceiveBeginPlay`
  (bind _returnvalue (pcsubsystem `EnhancedInputLocalPlayerSubsystem` self))
  (`/Engine/EditorBlueprintResources/StandardMacros.IsValid` _returnvalue
    (:`Is Valid`
      (`EnhancedInputSubsystemInterface.AddMappingContext` _returnvalue "/Game/CatBase/Input/IMC_Menu.IMC_Menu" 0 (struct))
      (`WidgetBlueprintLibrary.SetFocusToGameViewport`))))

(event `EnhancedInput|/Game/CatBase/Input/Actions/IA_Menu`
  (params (ActionValue :type Boolean) (ElapsedSeconds :type "Float (double-precision)") (TriggeredSeconds :type "Float (double-precision)") (InputAction :type "InputAction Object Reference" :default "/Game/CatBase/Input/Actions/IA_Menu.IA_Menu"))
  ;[1 1 1] Пауза
  (:`Started`
    (if (`GameplayStatics.IsGamePaused`)
      (`self.UnpauseMenu`)
      (else
        (`GameplayStatics.SetGamePaused` true)
        (`self.PauseMenu`)))))

(event `PauseMenu`
  (bind _pausewidget (`self.PauseWidget`))
  ;[1 1 1] Пауза
  (bind _returnvalue (`|CreateWidget` "/Game/CatBase/Blueprints/Widgets/WBP_PauseMenu.WBP_PauseMenu_C" self))
  (set `self.PauseWidget` _returnvalue)
  (`UserWidget.AddToViewport` _returnvalue 0)
  (`self.SetMode` true)
  (add `/Game/CatBase/Blueprints/Widgets/WBP_PauseMenu.Continue` _pausewidget (delegate `UnpauseMenu`))
  (add `/Game/CatBase/Blueprints/Widgets/WBP_PauseMenu.Restart` _pausewidget (delegate `Restart_Event`)))

(event `UnpauseMenu`
  ;[1 1 1] Пауза
  (`Widget.RemoveFromParent` (`self.PauseWidget`))
  (`self.SetMode` false)
  (`GameplayStatics.SetGamePaused` false))

(event `Restart_Event`
  ;[1 1 1] Пауза
  (`self.SetMode` false)
  (message `/Game/CatBase/Blueprints/BlueprintInterfaces/BPI_GMode.RestartEvent` (`GameplayStatics.GetGameMode`)))

(event `SetMode`
  (params (`setUI?` :type Boolean))
  ;[1 1 1] Пауза
  (if `setUI?`
    (set `self.bShowMouseCursor` true)
    (`WidgetBlueprintLibrary.SetInputMode_GameAndUIEx` self (`self.PauseWidget`) "DoNotLock" false)
    (else
      (set `self.bShowMouseCursor` false)
      (`WidgetBlueprintLibrary.SetInputMode_GameOnly` self))))

(fn `UserConstructionScript`)