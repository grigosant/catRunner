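; BP_Obstacle is a ghost-material obstacle that changes appearance as actors approach and deals type-based damage on contact.
; Its proximity box plays or reverses a timeline driving a dynamic material's GhostParameter, and starts or stops transform tracing on the actor via messages.
; The mesh's first overlap applies damage, sends forward-transform and stop-tracing messages, and plays sound; pawns leaving receive back-transform.
; Construction optionally sizes mesh and box.
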(event `self.ReceiveBeginPlay`
  (`self.CreateDynamicMaterial`))

(event `self.Box.OnComponentBeginOverlap`
  (params (OverlappedComponent :type "PrimitiveComponent Object Reference") (OtherActor :type "Actor Object Reference") (OtherComp :type "PrimitiveComponent Object Reference") (OtherBodyIndex :type Integer) (bFromSweep :type Boolean) (SweepResult :type "HitResult Structure (by ref)"))
  ;[1 1 1] переключение прозрачности при приближении
  (`self.ColorIncreases`)
  (message `/Game/CatBase/Blueprints/BlueprintInterfaces/BPI_Cat.StartTransformTracing` OtherActor))

(event `self.Box.OnComponentEndOverlap`
  (params (OverlappedComponent :type "PrimitiveComponent Object Reference") (OtherActor :type "Actor Object Reference") (OtherComp :type "PrimitiveComponent Object Reference") (OtherBodyIndex :type Integer))
  ;[1 1 1] переключение прозрачности при приближении
  (`self.ColorDecrease`)
  (message `/Game/CatBase/Blueprints/BlueprintInterfaces/BPI_Cat.StopTransformTracing` OtherActor))

(event `ColorIncreases`
  ;[1 1 1] переключение прозрачности при приближении
  (bind (_direction _newtrack_0) (`Timeline|Timeline` :!via `PlayFromStart` :!label _label)
    (:`Update`
      (`MaterialInstanceDynamic.SetScalarParameterValue` (`self.MeshMaterial`) "GhostParameter" (`KismetMathLibrary.MapRangeClamped` _newtrack_0 0.0 1.0 0.0 1.0)))))

(event `ColorDecrease`
  ;[1 1 1] переключение прозрачности при приближении
  (goto _label :!via `ReverseFromEnd`))

(event `self.StaticMesh.OnComponentBeginOverlap`
  (params (OverlappedComponent :type "PrimitiveComponent Object Reference") (OtherActor :type "Actor Object Reference") (OtherComp :type "PrimitiveComponent Object Reference") (OtherBodyIndex :type Integer) (bFromSweep :type Boolean) (SweepResult :type "HitResult Structure (by ref)"))
  ;[1 1 1] Нанесение урона при соприкосновении
  (`/Engine/EditorBlueprintResources/StandardMacros.DoOnce` false
    (:`Completed`
      (`GameplayStatics.ApplyDamage` OtherActor (`/Game/CatBase/Blueprints/BPL_Library.FindDamage` (`self.Type`)) null self)
      (message `/Game/CatBase/Blueprints/BlueprintInterfaces/BPI_Cat.ForwardTransform` OtherActor)
      (message `/Game/CatBase/Blueprints/BlueprintInterfaces/BPI_Cat.StopTransformTracing` OtherActor)
      (`GameplayStatics.SpawnSoundAtLocation` (select `/Game/CatBase/Blueprints/Data/E_DamageTypes` (`self.Type`) :`NewEnumerator2` "/Game/CatBase/Sounds/SW_short.SW_short" :`NewEnumerator3` "/Game/CatBase/Sounds/SW_long.SW_long" :!type "SoundBase Object Reference") (`self.K2_GetActorLocation`) (struct) 1.0 1.0 0.0 null null))))

(event `self.StaticMesh.OnComponentEndOverlap`
  (params (OverlappedComponent :type "PrimitiveComponent Object Reference") (OtherActor :type "Actor Object Reference") (OtherComp :type "PrimitiveComponent Object Reference") (OtherBodyIndex :type Integer))
  ;[1 1 1] Нанесение урона при соприкосновении
  (bind _aspawn (cast `Pawn` OtherActor))
  (message `/Game/CatBase/Blueprints/BlueprintInterfaces/BPI_Cat.BackTransform` _aspawn))

(fn `CreateDynamicMaterial`
  ;[1 1 1] Переключаемый призрачный материал
  (bind _returnvalue (`KismetMaterialLibrary.CreateDynamicMaterialInstance` "/Game/CatBase/Materials/MI_Ghost1.MI_Ghost1"))
  (bind _output_get (set `self.MeshMaterial` _returnvalue))
  (`PrimitiveComponent.SetMaterial` (`self.StaticMesh`) 0 _output_get)
  (`MaterialInstanceDynamic.SetScalarParameterValue` (`self.MeshMaterial`) "GhostParameter" 0.0))

(fn `SetupSize`
  (if (`self.CustomSetupSize`)
    (`SceneComponent.SetWorldScale3D` (`self.StaticMesh`) (`KismetMathLibrary.MakeVector` (`KismetMathLibrary.Conv_IntToDouble` (`self.sizeX`)) (`KismetMathLibrary.Conv_IntToDouble` (`self.sizeY`)) 1.0))
    (`SceneComponent.SetWorldScale3D` (`self.Box`) (`KismetMathLibrary.MakeVector` (`KismetMathLibrary.Conv_IntToDouble` (* (`self.sizeX`) (`self.CollisionX`))) (`KismetMathLibrary.Conv_IntToDouble` (* (`self.sizeY`) (`self.CollisionY`))) 2.0))
    (`SceneComponent.K2_SetWorldLocation` (`self.Box`) (`PrimitiveComponent.GetCenterOfMass` (`self.StaticMesh`) "None") false false)))

(fn `UserConstructionScript`
  (`self.SetupSize`))