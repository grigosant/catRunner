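; BPC_Health is an actor component that tracks its owner's health and signals death.
; On BeginPlay it fills Health to MaxHealth and binds to the owner's OnTakeAnyDamage, applying only damage whose DamageCauser is the owner itself.
; AdjustDamage subtracts the amount, clamps Health between zero and MaxHealth, and calls the Death dispatcher at zero.
; Getter functions expose current and maximum health.
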(event `self.ReceiveBeginPlay`
  (set `self.Health` (`self.MaxHealth`))
  (bind _output_get (set `self.Ownew` (`self.GetOwner`)))
  (add `Actor.OnTakeAnyDamage` _output_get (delegate `OnTakeAnyDamage_Event`)))

(event `OnTakeAnyDamage_Event`
  (params (DamagedActor :type "Actor Object Reference") (Damage :type "Float (single-precision)") (DamageType :type "DamageType Object Reference") (InstigatedBy :type "Controller Object Reference") (DamageCauser :type "Actor Object Reference"))
  (if (== DamageCauser (`self.Ownew`))
    (`self.AdjustDamage` Damage)))

(event `AdjustDamage`
  (params (Damage :type "Float (double-precision)"))
  (bind _output_get (set `self.Health` (`KismetMathLibrary.FClamp` (- (`self.Health`) Damage) 0.0 (`self.MaxHealth`))))
  (if (<= _output_get 0.0)
    (`self.Death`)))

(fn `GetCurrentHealth`
  (returns (Health :type "Float (double-precision)"))
  (return (`self.Health`)))

(fn `GetMaxHealth`
  (returns (Health :type "Float (double-precision)"))
  (return (`self.MaxHealth`)))