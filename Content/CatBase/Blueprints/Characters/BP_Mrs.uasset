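; BP_Mrs is an AI-controlled character that, on a StartMoving event, runs to the road and then along it.
; At BeginPlay it takes the first line position from the game mode as its target Y coordinate.
; StartMoving uses SimpleMoveToLocation to reach that Y, then a one-shot ReceiveMoveCompleted binding sends it a fixed distance along negative X.
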(event `self.ReceiveBeginPlay`
  (bind _ycoords (message `/Game/CatBase/Blueprints/BlueprintInterfaces/BPI_GMode.GetLinePositions` (`GameplayStatics.GetGameMode`)))
  (set `self.DesiredRotationPosition` (`|GetArrayItem` _ycoords)))

(event `/Game/CatBase/Blueprints/BlueprintInterfaces/BPI_Owner.StartMoving`
  (bind (_returnvalue_x _returnvalue_y _returnvalue_z) (`KismetMathLibrary.BreakVector` (`self.K2_GetActorLocation`)))
  (bind _returnvalue (`AIBlueprintHelperLibrary.GetAIController` self))
  ;[1 1 1] бежит к дороге...
  (`AIBlueprintHelperLibrary.SimpleMoveToLocation` _returnvalue (`KismetMathLibrary.MakeVector` _returnvalue_x (`self.DesiredRotationPosition`) _returnvalue_z))
  (add `AIController.ReceiveMoveCompleted` _returnvalue (delegate `ReceiveMoveCompleted_Event`)))

(event `ReceiveMoveCompleted_Event`
  (params (RequestID :type "AIRequestID Structure") (Result :type "EPathFollowingResult Enum" :default "Success"))
  (bind (_returnvalue_x _returnvalue_y _returnvalue_z) (`KismetMathLibrary.BreakVector` (`self.K2_GetActorLocation`)))
  ;[1 1 1] и бежит вдоль дороги
  (remove `AIController.ReceiveMoveCompleted` (`AIBlueprintHelperLibrary.GetAIController` self) (delegate `ReceiveMoveCompleted_Event`))
  (`AIBlueprintHelperLibrary.SimpleMoveToLocation` (`AIBlueprintHelperLibrary.GetAIController` self) (`KismetMathLibrary.MakeVector` (- _returnvalue_x 1500.0) _returnvalue_y _returnvalue_z)))

(fn `UserConstructionScript`)